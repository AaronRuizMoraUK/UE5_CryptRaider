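; BP_Player is the player Blueprint in CryptRaider and handles grabbing through its Grabber component.
; The Enhanced Input action IA_Grab works as a toggle, calling Release when the Grabber is already holding something and Grab otherwise.
; An unconnected hold-style variant, which grabs on a true value and releases on false, remains in the graph but never runs.
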(event `EnhancedInput|/Game/CryptRaider/Input/IA_Grab`
  (params (ActionValue :type Boolean) (ElapsedSeconds :type "Float (double-precision)") (TriggeredSeconds :type "Float (double-precision)") (InputAction :type "InputAction Object Reference" :default "/Game/CryptRaider/Input/IA_Grab.IA_Grab"))
  (bind _grabber (`self.Grabber`))
  (:`Triggered`
    (if ActionValue
      (if (`Grabber.IsGrabbing` _grabber)
        (`Grabber.Release` _grabber)
        (else
          (`Grabber.Grab` _grabber))))))

(fn `UserConstructionScript`
  (`parent.UserConstructionScript`))